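; BallGameMode is a game mode that keeps the score and runs a timed HORSE event.
; Starting the event resets the next letter and win flag, shows the HORSE_UI widget and begins a countdown.
; A self-rescheduling 0.1-second timer decrements the time left until it expires or HorseWin is set.
; Ending the event removes the widget, after a short delay on a win.
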(event Custom|Horse_Event_Start
  (Variables|Horse_Mode|SetNextLetter "NewEnumerator0")
  (Variables|Horse_Mode|SetHorseWin false)
  (CallFunction|HorseTimerEvent)
  (bind _returnvalue (UserInterface|CreateWidget "/Game/Blueprints/HorseEvent/HORSE_UI.HORSE_UI_C" (Game|GetPlayerController 0)))
  (UserInterface|Viewport|AddtoViewport _returnvalue 0))

(event Custom|HorseTimerEvent
  (bind _output_get (Variables|Horse_Mode|SetHorseTimeLeft (- (Variables|Horse_Mode|GetHorseTimeLeft) 0.1)))
  (if (and (> _output_get 0.0) (not (Variables|Horse_Mode|GetHorseWin)))
    (Utilities|Time|SetTimerbyEvent (delegate Custom|HorseTimerEvent) 0.1)
    (else
      (CallFunction|HorseEventEnd))))

(event Custom|Horse_Event_End
  (if (Variables|Horse_Mode|GetHorseWin)
    (Utilities|FlowControl|Delay 3.0))
  (Widget|RemovefromParent (stale Custom|Horse_Event_Start _returnvalue)))

(event EventBeginPlay)

(event EventTick
  (params (DeltaSeconds :type Float%20%28single-precision%29)))

(fn ConstructionScript)

(fn IncreaseScore
  (params (ChangeInScore :type Integer))
  (Variables|Default|SetScore (+ ChangeInScore (Variables|Default|GetScore))))

(fn GetScore
  (return (Variables|Default|GetScore)))