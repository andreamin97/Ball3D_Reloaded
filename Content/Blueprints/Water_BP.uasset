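; Water volume actor that applies a buoyancy-style force to the Ball_4 actor while it is inside the Box trigger.
; On begin overlap it stores the ball, enables the force and damps the ball's vertical velocity once.
; Each Tick adds ForceToApply minus the ball's height offset from the water actor's origin on Z.
; Any end overlap on the box switches the force off, regardless of which actor left.
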(event OnComponentBeginOverlap(Box)
  (params (OverlappedComponent :type Primitive%20Component%20Object%20Reference) (OtherActor :type Actor%20Object%20Reference) (OtherComp :type Primitive%20Component%20Object%20Reference) (OtherBodyIndex :type Integer) (bFromSweep :type Boolean) (SweepResult :type Hit%20Result%20Structure%20%28by%20ref%29))
  (bind _asball_4 (Utilities|Casting|CastToBall_4 OtherActor))
  (Variables|Default|SetAddImpulseToPlayer true)
  (bind _returnvalue (Physics|GetPhysicsLinearVelocity (Variables|/Game/Blueprints/Ball_4.Ball_4_C|GetSphere _asball_4) "None"))
  (Physics|SetPhysicsLinearVelocity (Variables|/Game/Blueprints/Ball_4.Ball_4_C|GetSphere _asball_4) (Math|Vector|MakeVector (.x _returnvalue) (.y _returnvalue) (* (.z _returnvalue) 0.6)) false "None"))

(event OnComponentEndOverlap(Box)
  (params (OverlappedComponent :type Primitive%20Component%20Object%20Reference) (OtherActor :type Actor%20Object%20Reference) (OtherComp :type Primitive%20Component%20Object%20Reference) (OtherBodyIndex :type Integer))
  (Variables|Default|SetAddImpulseToPlayer false))

(event EventBeginPlay)

(event Collision|EventActorBeginOverlap
  (params (OtherActor :type Actor%20Object%20Reference)))

(event EventTick
  (params (DeltaSeconds :type Float%20%28single-precision%29))
  (if (Variables|Default|GetAddImpulseToPlayer)
    (Physics|AddForce (Variables|/Game/Blueprints/Ball_4.Ball_4_C|GetSphere (stale OnComponentBeginOverlap(Box) _asball_4)) (- (Variables|Default|GetForceToApply) (Math|Vector|MakeVector 0.0 0.0 (.z (- (Transformation|GetWorldLocation (Variables|/Game/Blueprints/Ball_4.Ball_4_C|GetSphere (stale OnComponentBeginOverlap(Box) _asball_4))) (Transformation|GetActorLocation))))) "None" false)))

(fn ConstructionScript)